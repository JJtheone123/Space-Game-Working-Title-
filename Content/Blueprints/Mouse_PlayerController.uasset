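; Mouse-driven player controller for a turn-based, team-based tactics game played on a Board actor.
; Left clicks trace under the cursor to select a current-team unit, act on a clicked unit's tile, or move along an A* path.
; Selection state drives the SelectedUnit widget.
; Space cycles teams and resets the outgoing units; after a successful action, the turn auto-advances if the team is done.
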(event EventBeginPlay
  (bind _outactors (Actor|GetAllActorsOfClass "/Game/Blueprints/Board.Board_C"))
  (bind _output_get (Variables|Default|SetBoard (Utilities|Array|Get(acopy) _outactors)))
  (Variables|Default|SetTurn (Utilities|Array|Get(acopy) (Default|GetTeams _output_get)))
  (bind _returnvalue (UserInterface|CreateWidget "/Game/Blueprints/SelectedUnitWidget.SelectedUnitWidget_C"))
  (bind _output_get_2 (Variables|Default|SetUnit%20Widget _returnvalue))
  (UserInterface|Viewport|AddtoViewport _output_get_2 0))

(event Input|MouseEvents|LeftMouseButton
  (params (Key :type Key%20Structure))
  (:Released
    (CallFunction|OnClick)))

(event Input|KeyboardEvents|SpaceBar
  (params (Key :type Key%20Structure))
  (:Released
    (CallFunction|AdvanceTurn)))

(fn ConstructionScript)

(fn GameTurn
  (CallFunction|AdvanceTurn))

(fn AdvanceTurn
  (bind _board (Variables|Default|GetBoard))
  (bind _board_2 (Variables|Default|GetBoard))
  (bind _teams (Default|GetTeams _board_2))
  (bind _number_of_teams (Default|GetNumberOfTeams _board))
  (if (> _number_of_teams 1)
    (for _array_element (.Units (Default|GetUnitsfromTeam (Variables|Default|GetBoard) (Variables|Default|GetTurn)))
      (Variables|/Game/Blueprints/Unit.Unit_C|SetHas%20Attacked _array_element false)
      (Variables|/Game/Blueprints/Unit.Unit_C|SetAction%20Points _array_element (Variables|/Game/Blueprints/Unit.Unit_C|GetMax%20Action%20Points _array_element)))
    (if (== (Default|GetNumberOfTeams (Variables|Default|GetBoard)) (+ (Utilities|Array|FindItem _teams (Variables|Default|GetTurn)) 1))
      (Variables|Default|SetTurn (Utilities|Array|Get(acopy) _teams))
      (Development|PrintString (Utilities|String|BuildString(Integer) "" "Turn of team " (Variables|Default|GetTurn)))
      (else
        (Variables|Default|SetTurn (Utilities|Array|Get(acopy) _teams (+ (Utilities|Array|FindItem _teams (Variables|Default|GetTurn)) 1)))))
    (else
      (Development|PrintString "ERR: Not enough teams")
      (Development|PrintString (Utilities|String|BuildString(Integer) "" "Number of teams: " _number_of_teams)))))

(fn OnClick
  (bind (_hitresult _returnvalue) (Game|Player|GetHitResultUnderCursorbyChannel "TraceTypeQuery1" true))
  (bind _selected_unit (Variables|Default|GetSelected%20Unit))
  (bind _board (Variables|Default|GetBoard))
  (bind _board_2 (Variables|Default|GetBoard))
  (bind _selected_unit_2 (Variables|Default|GetSelected%20Unit))
  (bind _board_3 (Variables|Default|GetBoard))
  (bind (_board_x _board_y) (Default|GetPositiononBoard _selected_unit))
  (bind (_bblockinghit _binitialoverlap _time _distance _location _impactpoint _normal _impactnormal _physmat _hitactor) (Collision|BreakHitResult _hitresult))
  (bind _returnvalue_2 (Math|Conversions|ToFloat(Integer) _board_x))
  (bind _returnvalue_3 (Math|Conversions|ToFloat(Integer) _board_y))
  (bind (_board_x_2 _board_y_2) (Default|WorldtoBoardLocation _board _location))
  (bind (_board_x_3 _board_y_3) (Default|WorldtoBoardLocation _board_3 _location))
  (bind _returnvalue_4 (Math|Conversions|ToFloat(Integer) _board_x_2))
  (bind _returnvalue_5 (Math|Conversions|ToFloat(Integer) _board_y_2))
  (bind _returnvalue_6 (Math|Vector2D|MakeVector2D _returnvalue_2 _returnvalue_3))
  (bind _returnvalue_7 (Math|Vector2D|MakeVector2D _returnvalue_4 _returnvalue_5))
  (bind (_path _success) (CallFunction|AStar _board_2 _returnvalue_6 _returnvalue_7))
  (if _returnvalue
    ;[1 1 1] If the user clicked on a unit...
    (if (== (Utilities|GetClass _hitactor) "/Game/Blueprints/Unit.Unit_C")
      ;[1 1 1] If there's a selected unit...
      (if (Variables|Default|GetHas%20Selected%20Unit)
        ;[1 1 1] Try making the unit do something on the clicked cell.
        (bind _could_act (Default|ActUponTile _board_3 _board_x_3 _board_y_3 _selected_unit_2))
        (if _could_act
          (CallFunction|DeselectUnit)
          (Variables|/Game/Blueprints/Unit.Unit_C|SetHas%20Attacked _selected_unit_2 _could_act)
          (CallFunction|AutoAdvance))
        (else
          ;[1 1 1] Else, try selecting a unit.
          (bind _asunit (Utilities|Casting|CastToUnit _hitactor))
          (CallFunction|TrySelectUnit _asunit)))
      (else
        ;[1 1 1] Else if the user clicked on the board and there's a unit selected...
        (if (and (== (Utilities|GetClass _hitactor) "/Game/Blueprints/Board.Board_C") (Variables|Default|GetHas%20Selected%20Unit))
          ;[1 1 1] If a path was found...
          (if _success
            ;[1 1 1] Move the unit
            (Default|MoveonBoard (Variables|Default|GetSelected%20Unit) _path)
            (CallFunction|DeselectUnit)
            (else
              ;[1 1 1] Else, print an error.
              (Development|PrintString "Couldn't find path"))))))
    (elif (Variables|Default|GetHas%20Selected%20Unit)
      (Variables|Default|SetHas%20Selected%20Unit false)
      (Development|PrintString "Deselected Unit (Clicked on nothing)"))))

(fn AutoAdvance
  (bind _array_element (Utilities|Array|ForEachLoopwithBreak (.Units (Default|GetUnitsfromTeam (Variables|Default|GetBoard) (Variables|Default|GetTurn))) :!label _label)
    (:LoopBody
      (if (not (Default|IsDonewithTurn _array_element))
        (goto _label Break)))
    (:Completed
      (if (Default|IsDonewithTurn _array_element)
        (Development|PrintString "Automatically advancing to next turn...")
        (CallFunction|AdvanceTurn)))))

(fn UnitIsSelectable
  (params (Unit :type Unit%20Object%20Reference))
  (return (and (not (Variables|/Game/Blueprints/Unit.Unit_C|GetHas%20Attacked Unit)) (Utilities|Array|ContainsItem (.Units (Default|GetUnitsfromTeam (Variables|Default|GetBoard) (Variables|Default|GetTurn))) Unit))))

(fn DeselectUnit
  (Variables|Default|SetHas%20Selected%20Unit false)
  (Default|UnitDeselected (Variables|Default|GetUnit%20Widget))
  (Development|PrintString "Deselected"))

(fn TrySelectUnit
  (params (Unit :type Unit%20Object%20Reference))
  (bind _selectable (CallFunction|UnitIsSelectable Unit))
  (bind _unit_widget (Variables|Default|GetUnit%20Widget))
  (if _selectable
    (Variables|Default|SetHas%20Selected%20Unit true)
    (bind _output_get (Variables|Default|SetSelected%20Unit Unit))
    (Default|UnitSelected _unit_widget _output_get)
    (else
      (Default|SelectFailed _unit_widget)))
  (Development|PrintString "Tried Select")
  (return _selectable))