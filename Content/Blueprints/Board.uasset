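; Grid board for a team-based unit game, with its tile meshes generated in the construction script from width, height, cell size and margin.
; Helpers convert between world and cell coordinates relative to world origin, clamping only on the board-to-world side.
; Occupancy and team queries scan the Units array.
; ActUponTile uses occupancy to subtract the actor's attack points from a hated occupant's health.
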(fn ConstructionScript
  (bind _board_cell_margin (Variables|Default|GetBoard%20Cell%20Margin))
  (bind _board_cell_size (Variables|Default|GetBoard%20Cell%20Size))
  (bind _returnvalue (+ _board_cell_size _board_cell_margin))
  (for _index (range 0 (- (Variables|Default|GetHeight) 1))
    (for _index_2 (range 0 (- (Variables|Default|GetWidth) 1))
      (AddComponent|AddStaticMeshComponent false (Math|Transform|MakeTransform (Math|Vector|MakeVector (* (Math|Conversions|ToFloat(Integer) _index_2) _returnvalue) (* (Math|Conversions|ToFloat(Integer) _index) _returnvalue) 0.0) "0, 0, 0" (Math|Conversions|ToVector(Float) (/ (Variables|Default|GetBoard%20Cell%20Size) 1e+02)))))))

(fn WorldtoBoardLocation
  (params (World%20Location :type Vector))
  (bind _board_cell_size (Variables|Default|GetBoard%20Cell%20Size))
  (bind _board_cell_margin (Variables|Default|GetBoard%20Cell%20Margin))
  (bind _board_cell_size_2 (Variables|Default|GetBoard%20Cell%20Size))
  (bind _returnvalue (/ _board_cell_size 2.0))
  (bind _returnvalue_2 (+ _board_cell_size_2 _board_cell_margin))
  (bind _returnvalue_3 (Math|Vector|MakeVector _returnvalue _returnvalue 0.0))
  (bind _returnvalue_4 (+ World%20Location _returnvalue_3))
  (bind _returnvalue_5 (/ _returnvalue_4 _returnvalue_2))
  (bind (_x _y) (Math|Vector|BreakVector _returnvalue_5))
  (return (Math|Float|Floor _x) (Math|Float|Floor _y)))

(fn BoardtoWorldLocation
  (params (Board%20X :type Integer) (Board%20Y :type Integer))
  (return (* (Math|Vector|MakeVector (Math|Conversions|ToFloat(Integer) (Math|Integer|Min(Integer) (Math|Integer|Max(Integer) Board%20X) (- (Variables|Default|GetWidth) 1))) (Math|Conversions|ToFloat(Integer) (Math|Integer|Min(Integer) (Math|Integer|Max(Integer) Board%20Y) (- (Variables|Default|GetHeight) 1))) 0.0) (+ (Variables|Default|GetBoard%20Cell%20Size) (Variables|Default|GetBoard%20Cell%20Margin)))))

(fn CellIsOccupiedbyUnit
  (params (Board%20X :type Integer) (Board%20Y :type Integer))
  (bind _array_element (Utilities|Array|ForEachLoopwithBreak (Variables|Default|GetUnits) :!label _label)
    (:LoopBody
      (if (and (== (.Board%20Y (Default|GetPositiononBoard _array_element)) Board%20Y) (== Board%20X (.Board%20X (Default|GetPositiononBoard _array_element))))
        (goto _label Break)))
    (:Completed
      (return (and (== (.Board%20Y (Default|GetPositiononBoard _array_element)) Board%20Y) (== Board%20X (.Board%20X (Default|GetPositiononBoard _array_element)))) _array_element))))

(fn ActUponTile
  (params (Board%20X :type Integer) (Board%20Y :type Integer) (Actor :type Unit%20Object%20Reference))
  (bind (_is_occupied _unit) (CallFunction|GetCellOccupant Board%20X Board%20Y))
  (if _is_occupied
    (if (Default|HatesUnit Actor _unit)
      (Variables|/Game/Blueprints/Unit.Unit_C|SetHealth%20Points _unit (- (Variables|/Game/Blueprints/Unit.Unit_C|GetHealth%20Points _unit) (Variables|/Game/Blueprints/Unit.Unit_C|GetAttack%20points Actor)))
      (Development|PrintString "Unit attacked.")
      (return true)
      (else
        (Development|PrintString "Cannot act, target is friend or actor is neutral")
        (Development|PrintString (Utilities|String|BuildString(Integer) "" "Team " (Variables|/Game/Blueprints/Unit.Unit_C|GetTeam Actor) (Utilities|String|BuildString(Integer) "" "== Team " (Variables|/Game/Blueprints/Unit.Unit_C|GetTeam _unit))))))
    (else
      (Development|PrintString "Cannot act, cell is empty")))
  (return false))

(fn GetCellOccupant
  (params (Board%20X :type Integer) (Board%20Y :type Integer))
  (bind (_is_occpuied _unit_) (CallFunction|CellIsOccupiedbyUnit Board%20X Board%20Y))
  (return _is_occpuied _unit_))

(fn GetTeams
  (for _array_element (Variables|Default|GetUnits)
    (Utilities|Array|AddUnique (LocalVariables|GetRes) (Variables|/Game/Blueprints/Unit.Unit_C|GetTeam _array_element)))
  (bind _sorted_array (CallFunction|SortIntegerArray (LocalVariables|GetRes)))
  (return _sorted_array))

(fn GetNumberOfTeams
  (return (Utilities|Array|Length (CallFunction|GetTeams))))

(fn GetUnitsfromTeam
  (params (Team :type Integer))
  (bind _result (LocalVariables|GetResult))
  (for _array_element (Variables|Default|GetUnits)
    (if (== (Variables|/Game/Blueprints/Unit.Unit_C|GetTeam _array_element) Team)
      (Utilities|Array|Add (LocalVariables|GetResult) _array_element)))
  (return (> (Utilities|Array|Length _result) 0) _result))