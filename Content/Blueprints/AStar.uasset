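; Blueprint A* pathfinder that searches a Board grid between two 2D points, returning the path and a success flag.
; AStar expands the open set via GetNeighbours, which yields eight-way cells absent from the Board's obstacles, and ReconstructPath backtracks through CameFrom.
; GetHeuristic gives straight-line distance.
; The step cost measures each neighbour against itself, so G stays zero, and the minimum F is never reset between iterations.
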(fn AStar
  (params (Board :type Board%20Object%20Reference) (Start :type Vector%202D%20Structure) (End :type Vector%202D%20Structure))
  ;[1 1 1] Initialization
  (Utilities|Set|Add (LocalVariables|GetOpen%20Set) Start)
  (Utilities|Map|Add (LocalVariables|GetGScore) Start 0.0)
  (Utilities|Map|Add (LocalVariables|GetFScore) Start (CallFunction|GetHeuristic Start End))
  ;[1 1 1] While the open set has elements...
  (while (!= (Utilities|Set|Length (LocalVariables|GetOpen%20Set)) 0)
    ;[1 1 1] Find the element with the lowest F score and set current to it.
    (bind _result (Utilities|Set|ToArray (LocalVariables|GetOpen%20Set)))
    (for _array_element _result
      (if (< (.Value (Utilities|Map|Find (LocalVariables|GetFScore) _array_element)) (LocalVariables|GetMin%20FScore))
        (LocalVariables|SetMin%20FScore (.Value (Utilities|Map|Find (LocalVariables|GetFScore) _array_element)))
        (LocalVariables|SetMin%20Node _array_element)))
    (LocalVariables|SetCurrent (LocalVariables|GetMin%20Node))
    ;[1 1 1] Move the current node from the open set to the closed set.
    (Utilities|Set|Remove (LocalVariables|GetOpen%20Set) (LocalVariables|GetCurrent))
    (Utilities|Set|Add (LocalVariables|GetClosed%20Set) (LocalVariables|GetCurrent))
    ;[1 1 1] If we are currently at the goal node...
    (if (Math|Vector|Equal(Vector) End (LocalVariables|GetCurrent) 0.0001)
      ;[1 1 1] Reconstruct the path and return successfully.
      (return (CallFunction|ReconstructPath (LocalVariables|GetCame%20From) (LocalVariables|GetCurrent)) true)
      (else
        ;[1 1 1] Else, for each neighbour...
        (for _array_element_2 (CallFunction|GetNeighbours (LocalVariables|GetCurrent) Board)
          (LocalVariables|SetNeighbour _array_element_2)
          ;[1 1 1] If it's in the closed set, do nothing, otherwise...
          (if (not (Utilities|Set|Contains (LocalVariables|GetClosed%20Set) (LocalVariables|GetNeighbour)))
            ;[1 1 1] If the node isn't inside the open set (it's a new node), add it.
            (if (not (Utilities|Set|Contains (LocalVariables|GetOpen%20Set) (LocalVariables|GetNeighbour)))
              (Utilities|Set|Add (LocalVariables|GetOpen%20Set) (LocalVariables|GetNeighbour)))
            ;[1 1 1] Set the "Tentative GScore"
            (LocalVariables|SetTentative%20GScore (+ (.Value (Utilities|Map|Find (LocalVariables|GetGScore) (LocalVariables|GetCurrent))) (CallFunction|GetHeuristic _array_element_2 (LocalVariables|GetNeighbour))))
            ;[1 1 1] If the tentative g-score is better than what the neighbour already has...
            (if (< (LocalVariables|GetTentative%20GScore) (Math|Float|SelectFloat (.Value (Utilities|Map|Find (LocalVariables|GetFScore) (LocalVariables|GetNeighbour))) 1e+07 (.ReturnValue (Utilities|Map|Find (LocalVariables|GetFScore) (LocalVariables|GetNeighbour)))))
              ;[1 1 1] Add the neighbour, its g-score and its f-score to the appropriate places.
              (Utilities|Map|Add (LocalVariables|GetCame%20From) (LocalVariables|GetNeighbour) (LocalVariables|GetCurrent))
              (Utilities|Map|Add (LocalVariables|GetGScore) (LocalVariables|GetNeighbour) (LocalVariables|GetTentative%20GScore))
              (Utilities|Map|Add (LocalVariables|GetFScore) (LocalVariables|GetNeighbour) (+ (LocalVariables|GetTentative%20GScore) (CallFunction|GetHeuristic (LocalVariables|GetNeighbour) End)))))))))
  ;[1 1 1] If the loop finishes, a path couldn't be found - exit with failure
  (return (Utilities|Array|MakeArray "") false))

(fn GetHeuristic
  (params (Node :type Vector%202D%20Structure) (Goal :type Vector%202D%20Structure))
  (return (Math|Vector2D|Vector2DLength (- Node Goal))))

(fn ReconstructPath
  (params (Came%20From :type Map%20of%20Vector%202D%20Structures%20to%20Structs) (Current :type Vector%202D%20Structure))
  (LocalVariables|SetCurr Current)
  (Utilities|Array|Add (LocalVariables|GetTotal%20Path) (LocalVariables|GetCurr))
  ;[1 1 1] While the current node is inside the Came From map
  (while (.ReturnValue (Utilities|Map|Find Came%20From (LocalVariables|GetCurr)))
    (LocalVariables|SetCurr (.Value (Utilities|Map|Find Came%20From (LocalVariables|GetCurr))))
    (Utilities|Array|Insert (LocalVariables|GetTotal%20Path) (LocalVariables|GetCurr)))
  (return (LocalVariables|GetTotal%20Path)))

(fn GetNeighbours
  (params (Node :type Vector%202D%20Structure) (Board :type Board%20Object%20Reference%20%28by%20ref%29))
  (bind _returnvalue (+ Node "(X=-1.000000,Y=-1.000000)"))
  (bind _returnvalue_2 (+ Node "(X=-1.000000,Y=1.000000)"))
  (bind _returnvalue_3 (+ Node "(X=1.000000,Y=-1.000000)"))
  (bind _returnvalue_4 (+ Node "(X=0.000000,Y=1.000000)"))
  (bind _returnvalue_5 (+ Node "(X=0.000000,Y=-1.000000)"))
  (bind _returnvalue_6 (+ Node "(X=1.000000,Y=0.000000)"))
  (bind _returnvalue_7 (+ Node "(X=-1.000000,Y=0.000000)"))
  (bind _returnvalue_8 (+ Node "(X=1.000000,Y=1.000000)"))
  ;[1 1 1] Determine if node has a neighbour upwards
  (LocalVariables|SetUp (< (.Y (Math|Vector2D|BreakVector2D Node)) (Math|Conversions|ToFloat(Integer) (Variables|/Game/Blueprints/Board.Board_C|GetHeight Board))))
  ;[1 1 1] Determine if node has a neighbour downwards
  (LocalVariables|SetDown (> (.Y (Math|Vector2D|BreakVector2D Node)) 0.0))
  ;[1 1 1] Determine if node has a neighbour to its left
  (LocalVariables|SetLeft (< (.X (Math|Vector2D|BreakVector2D Node)) (Math|Conversions|ToFloat(Integer) (Variables|/Game/Blueprints/Board.Board_C|GetWidth Board))))
  ;[1 1 1] Determine if node has a neighbour to its right
  (LocalVariables|SetRight (> (.X (Math|Vector2D|BreakVector2D Node)) 0.0))
  ;[1 1 1] Add neighbour upwards (if one exists)
  (if (and (LocalVariables|GetUp) (not (CallFunction|IsObstructed _returnvalue_4 Board)))
    (Utilities|Array|Add (LocalVariables|GetResult) _returnvalue_4))
  ;[1 1 1] Add neighbour downwards (if one exists)
  (if (and (LocalVariables|GetDown) (not (CallFunction|IsObstructed _returnvalue_5 Board)))
    (Utilities|Array|Add (LocalVariables|GetResult) _returnvalue_5))
  ;[1 1 1] Add neighbour to the left (if one exists)
  (if (and (LocalVariables|GetLeft) (not (CallFunction|IsObstructed _returnvalue_6 Board)))
    (Utilities|Array|Add (LocalVariables|GetResult) _returnvalue_6))
  ;[1 1 1] Add neighbour to the right (if one exists)
  (if (and (LocalVariables|GetRight) (not (CallFunction|IsObstructed _returnvalue_7 Board)))
    (Utilities|Array|Add (LocalVariables|GetResult) _returnvalue_7))
  ;[1 1 1] Add neighbour diagonally up and left
  (if (Math|Boolean|ANDBoolean (LocalVariables|GetUp) (LocalVariables|GetLeft) (not (CallFunction|IsObstructed _returnvalue_8 Board)))
    (Utilities|Array|Add (LocalVariables|GetResult) _returnvalue_8))
  ;[1 1 1] Add neighbour diagonally up and right
  (if (Math|Boolean|ANDBoolean (LocalVariables|GetRight) (LocalVariables|GetUp) (not (CallFunction|IsObstructed _returnvalue_2 Board)))
    (Utilities|Array|Add (LocalVariables|GetResult) _returnvalue_2))
  ;[1 1 1] Add neighbour diagonally down and left
  (if (Math|Boolean|ANDBoolean (LocalVariables|GetDown) (LocalVariables|GetLeft) (not (CallFunction|IsObstructed _returnvalue_3 Board)))
    (Utilities|Array|Add (LocalVariables|GetResult) _returnvalue_3))
  ;[1 1 1] Add neighbour diagonally down and right
  (if (Math|Boolean|ANDBoolean (LocalVariables|GetDown) (LocalVariables|GetRight) (not (CallFunction|IsObstructed _returnvalue Board)))
    (Utilities|Array|Add (LocalVariables|GetResult) _returnvalue))
  ;[1 1 1] Return result
  (return (LocalVariables|GetResult)))

(fn IsObstructed
  (params (Node :type Vector%202D%20Structure) (Board :type Board%20Object%20Reference%20%28by%20ref%29))
  (return (Utilities|Array|ContainsItem (Default|GetObstacles Board) Node)))