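; Blueprint sorting utility with functions that return integer and float arrays in ascending order.
; Each uses a selection sort, repeatedly appending the minimum value to a result array and removing it by index from the input.
; The input array is emptied in the process, and the minimum search appears twice per iteration, giving quadratic cost.
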(fn SortIntegerArray
  (params (Array :type Array%20of%20Integers))
  (bind (_indexofminvalue _minvalue) (Math|Integer|MinOfIntArray Array))
  (while (> (Utilities|Array|Length Array) 0)
    (Utilities|Array|Add (LocalVariables|GetSorted%20array%20) _minvalue)
    (Utilities|Array|RemoveIndex Array _indexofminvalue))
  (return (LocalVariables|GetSorted%20array%20)))

(fn SortFloatArray
  (params (Array :type Array%20of%20Floats%20%28single-precision%29))
  (bind (_indexofminvalue _minvalue) (Math|Float|MinOfFloatArray Array))
  (while (> (Utilities|Array|Length Array) 0)
    (Utilities|Array|Add (LocalVariables|GetSorted%20array%20) _minvalue)
    (Utilities|Array|RemoveIndex Array _indexofminvalue))
  (return (LocalVariables|GetSorted%20array%20)))