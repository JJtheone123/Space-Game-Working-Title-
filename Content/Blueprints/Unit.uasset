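; Unit is a team-owned board-game piece with health and action points that lives on the level's Board actor.
; On BeginPlay it finds the Board, snaps to a cell and registers itself; if unnamed, it also sets name, full stats and team-colored material.
; Movement converts cells to world locations and rejects occupied ones.
; Helpers report position, life fraction and hostility, treating team zero as neutral and negative teams as hostile to all.
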(event EventBeginPlay
  (bind _staticmesh (Variables|Default|GetStaticMesh))
  (bind _outactors (Actor|GetAllActorsOfClass "/Game/Blueprints/Board.Board_C"))
  (bind _output_get (Variables|Default|SetBoard (Utilities|Array|Get(acopy) _outactors)))
  (CallFunction|SnaptoBoard)
  (Utilities|Array|Add (Variables|/Game/Blueprints/Board.Board_C|GetUnits _output_get) self)
  ;[1 1 1] Set name if one hasn't already been given
  (if (< (Utilities|String|Len (Variables|Default|GetName)) 1)
    (bind _output_get_2 (Variables|Default|SetName (Utilities|String|BuildString(Integer) "" "Tank " (Variables|Default|GetTeam))))
    (Development|PrintString _output_get_2)
    ;[1 1 1] Set current health to max
    (Variables|Default|SetHealth%20Points (Variables|Default|GetMax%20Health))
    ;[1 1 1] Set current Action Points to Max
    (Variables|Default|SetAction%20Points (Variables|Default|GetMax%20Action%20Points))
    ;[1 1 1] Set color based on team
    (switch int (Variables|Default|GetTeam)
      (:-1
        (Rendering|Material|SetMaterial _staticmesh 0 "/Game/Red.Red"))
      (:0
        (Rendering|Material|SetMaterial _staticmesh 0 "/Game/White.White"))
      (:1
        (Rendering|Material|SetMaterial _staticmesh 0 "/Game/Blue.Blue"))
      (:2
        (Rendering|Material|SetMaterial _staticmesh 0 "/Game/Green.Green")))))

(fn ConstructionScript)

(fn SnaptoBoard
  (bind _returnvalue (Transformation|GetActorLocation))
  (bind _board (Variables|Default|GetBoard))
  (bind (_board_x _board_y) (Default|WorldtoBoardLocation _board _returnvalue))
  (Transformation|SetActorLocation (Default|BoardtoWorldLocation _board _board_x _board_y) false false))

(fn MoveonBoard
  (params (Board%20X :type Integer) (Board%20Y :type Integer))
  (bind _board (Variables|Default|GetBoard))
  (bind _is_occpuied (Default|CellIsOccupiedbyUnit _board Board%20X Board%20Y))
  (if _is_occpuied
    (Development|PrintString "Can't move, cell is occupied")
    (else
      (Transformation|SetActorLocation (Default|BoardtoWorldLocation _board Board%20X Board%20Y) false false)
      (return _is_occpuied))))

(fn GetPositiononBoard
  (bind _returnvalue (Transformation|GetActorLocation))
  (bind _board (Variables|Default|GetBoard))
  (bind (_board_x _board_y) (Default|WorldtoBoardLocation _board _returnvalue))
  (return _board_x _board_y))

(fn IsNeutral
  (return (== (Variables|Default|GetTeam) 0)))

(fn IsCrazy
  (return (< (Variables|Default|GetTeam) 0)))

(fn HatesTeam
  (params (Team :type Integer))
  (if (CallFunction|IsNeutral)
    (return false)
    (elif (CallFunction|IsCrazy)
      (return true)
      (else
        (return (!= Team (Variables|Default|GetTeam)))))))

(fn HatesUnit
  (params (Unit :type Unit%20Object%20Reference))
  (return (CallFunction|HatesTeam (Variables|Unit_C|GetTeam Unit))))

(fn GetLifePercentage
  (return (/ (Variables|Default|GetHealth%20Points) (Variables|Default|GetMax%20Health))))